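; LobbyGM is the multiplayer lobby game mode, coordinating players from joining until the match starts.
; It tracks controllers on login and logout, then relays list refreshes, class initialization and chat through LobbyPC client calls.
; When at least two players are all ready, it shortens the LobbyGS countdown.
; Match start saves each player's settings, shows loading screens and server-travels to the map built from the game instance's mode and map index.
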(event Custom|E_UpdatePlayerLists
  ;[1 1 1] Update players lists on all clients
  (for _array_element (Variables|Default|GetAllPlayerControllers)
    (Default|CLGeneratePlayerLists (.AsLobby%20PC (Utilities|Casting|CastToLobbyPC _array_element)))))

(event Custom|SRV_AddChatMessage
  (params (SenderName :type String) (Message :type String) (SenderColor :type Slate%20Color%20Structure))
  ;[1 1 1] Add chat message in ChatBox on all clients
  (for _array_element (Variables|Default|GetAllPlayerControllers)
    (bind _aslobby_pc (Utilities|Casting|CastToLobbyPC _array_element))
    (Utilities|IsValid _aslobby_pc
      (:Is%20Valid
        (Default|CLGetChatMessage _aslobby_pc SenderName Message SenderColor)))))

(event Custom|E_IsAllReady
  (bind _returnvalue (Game|GetGameState))
  (bind _playerarray (Variables|/Script/Engine.GameStateBase|GetPlayerArray _returnvalue))
  ;[1 1 1] Check is All players are ready and if YES - set Minutes = 0 and seconds = 5 in GameState
  (bind _array_element (Utilities|Array|ForEachLoopwithBreak _playerarray :!label _label)
    (:LoopBody
      (bind _aslobby_ps (Utilities|Casting|CastToLobbyPS _array_element))
      (if (Variables|/Game/MP_SK/Blueprints/Lobby/LobbyPS.LobbyPS_C|GetIsReady _aslobby_ps)
        (Variables|Default|SetAllReady true)
        (else
          (Variables|Default|SetAllReady false)
          (goto _label Break))))
    (:Completed
      (if (and (Variables|Default|GetAllReady) (>= (Utilities|Array|Length _playerarray) 2))
        (bind _aslobby_gs (Utilities|Casting|CastToLobbyGS (Game|GetGameState)))
        (Variables|/Game/MP_SK/Blueprints/Lobby/LobbyGS.LobbyGS_C|Setminutes _aslobby_gs 0)
        (Variables|/Game/MP_SK/Blueprints/Lobby/LobbyGS.LobbyGS_C|Setseconds _aslobby_gs 5)))))

(event Custom|E_StartMatch
  ;[0 1 0.05329] Start Match
  (for _array_element (Variables|Default|GetAllPlayerControllers)
    (bind _aslobby_pc (Utilities|Casting|CastToLobbyPC _array_element))
    (Default|CLSavePlayerSettingsinGI _aslobby_pc)
    (Default|CLShowLobbyLoadingScreen _aslobby_pc))
  (Development|ExecuteConsoleCommand (CallFunction|FServerTraverCommand) (Game|GetPlayerController 0)))

(event Custom|E_InitPlayersClass
  ;[1 1 1] Init Class for everyone when updating server settings
  (Utilities|FlowControl|Delay 0.2)
  (for _array_element (Variables|Default|GetAllPlayerControllers)
    (bind _aslobby_pc (Utilities|Casting|CastToLobbyPC _array_element))
    (Default|CLInitClass _aslobby_pc)))

(event EventPostLogin
  (params (NewPlayer :type Player%20Controller%20Object%20Reference))
  ;[1 1 1] New Player PostLogIn. Updage Player Lists on all clients
  (Utilities|Array|Add (Variables|Default|GetAllPlayerControllers) NewPlayer)
  (Utilities|FlowControl|Delay 1.0)
  (CallFunction|EUpdatePlayerLists))

(event EventOnLogout
  (params (ExitingController :type Controller%20Object%20Reference))
  (bind _aslobby_pc (Utilities|Casting|CastToLobbyPC ExitingController))
  ;[1 1 1] Update Player Lists on all clients when some player Logout
  (Utilities|Array|RemoveItem (Variables|Default|GetAllPlayerControllers) _aslobby_pc)
  (if (== (Variables|/Game/MP_SK/Blueprints/Lobby/LobbyPS.LobbyPS_C|GetTeam (.AsLobby%20PS (Utilities|Casting|CastToLobbyPS (Variables|/Script/Engine.Controller|GetPlayerState _aslobby_pc)))) 0)
    (Variables|PlayersCount|SetRedTeamPlayersCount (- (Variables|PlayersCount|GetRedTeamPlayersCount) 1))
    (else
      (Variables|PlayersCount|SetBlueTeamPlayersCount (- (Variables|PlayersCount|GetBlueTeamPlayersCount) 1))))
  (Utilities|FlowControl|Delay 1.0)
  (CallFunction|EUpdatePlayerLists))

(fn ConstructionScript)

(fn FServerTraverCommand
  (bind _returnvalue (Game|GetGameInstance))
  (bind _asmain_gi (Utilities|Casting|CastToMainGI _returnvalue))
  (switch int (Variables|/Game/MP_SK/Blueprints/MainGI.MainGI_C|GetGameModeId _asmain_gi)
    (:Default
      (Variables|Default|SetGameModePath "TDM/" :!label _label))
    (:0
      (goto _label))
    (:1
      (Variables|Default|SetGameModePath "Classic/")))
  (return (Utilities|String|Append "servertravel /Game/MP_SK/Maps/" (Variables|Default|GetGameModePath) (.mapname (Utilities|Array|Get(acopy) (Utilities|Struct|BreakAllMapsStruct (Variables|Default|GetAllMapsStruct)) (Variables|/Game/MP_SK/Blueprints/MainGI.MainGI_C|GetIMapIndex _asmain_gi))))))