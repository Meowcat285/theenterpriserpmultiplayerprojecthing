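; BaseGS is a Blueprint Interface, apparently for the multiplayer Game State, exposing team-based round match state and events.
; It declares calls for round timing and completion, respawn countdowns, player kills and red ("Read") and blue team scores.
; Getters also expose server name, map index, game mode ID and friendly fire.
; It holds only signatures with default returns, leaving all logic to implementing classes.
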(fn IEUpdateTeamScore
  (params (Kiler%20Team :type Integer)))

(fn IFRoundFinished
  (return false))

(fn IFInitGameTime
  (return false))

(fn IERoundTimeCountDown
  (return))

(fn IFRoundTimeCountDown
  (return false))

(fn IERespawnCountDown)

(fn IEStartRespawnTimer)

(fn IFGetRoundSeconds
  (return 0))

(fn IFGetRoundMinutes
  (return 0))

(fn IFGetReadTeamScore
  (return 0))

(fn IFSetReadScore
  (params (new%20score :type Integer))
  (return 0))

(fn IFGetBlueTeamScore
  (return 0))

(fn IFSetBlueTeamScore
  (params (new%20score :type Integer))
  (return 0))

(fn IFGetRespawnDelaySeconds
  (return 0))

(fn IEPlayerKilled
  (params (Killed%20player%20Team :type Integer)))

(fn IFGetServerName
  (return ""))

(fn IFGetMapIndex
  (return 0))

(fn IFGetGameModeId
  (return 0))

(fn IFGetFriendlyFire
  (return false))