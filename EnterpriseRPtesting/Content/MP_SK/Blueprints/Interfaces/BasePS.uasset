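; BasePS is a Blueprint interface for multiplayer player data, apparently implemented by the player state.
; It declares getter and setter functions for team, class, health, score, kills and deaths.
; It also declares parameterless events to initialize health and grenade count and to update the score, kill and death counts.
; It holds only signatures, so all behavior comes from implementing classes.
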(fn IFSetTeam
  (params (Team :type Integer))
  (return 0))

(fn IFSetClass
  (params (ClassId :type Integer))
  (return 0))

(fn IFGetTeam
  (return 0))

(fn IFGetClass
  (return 0))

(fn IFGetHealth
  (return 0.0))

(fn IFSetHealth
  (params (Heatlh :type Float%20%28single-precision%29))
  (return 0.0))

(fn IEInitHealthandGrenadesCount)

(fn IEUpdateDeathsCount)

(fn IEUpdateKillsCount)

(fn IEUpdatePlayerScore)

(fn IFGetScore
  (return 0))

(fn IFSetScore
  (params (score :type Integer))
  (return 0))

(fn IFGetKills
  (return 0))

(fn IFSetKills
  (params (New%20kills :type Integer))
  (return 0))

(fn IFGetDeaths
  (return 0))

(fn IFSetDeaths
  (params (new%20deaths :type Integer))
  (return 0))