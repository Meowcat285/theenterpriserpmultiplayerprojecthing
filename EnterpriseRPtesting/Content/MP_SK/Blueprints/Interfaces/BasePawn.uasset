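; BasePawn is a Blueprint interface for pawns that carry weapons and can take damage and die.
; Its functions get and set the primary, secondary and equipped weapon.
; Its events signal damage with a bone name and torso damage value, death, picking up a dropped item, and dropping a weapon by type.
; It declares signatures only, leaving all logic to the implementing classes.
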(fn IFGetPrimaryWeapon
  (return 0))

(fn IFSetPrimaryWeapon
  (params (Primary%20Weapon :type A%20Base%20Weapon%20Object%20Reference))
  (return 0))

(fn IFSetEquipedWeapon
  (params (EquipedWeapon :type A%20Base%20Weapon%20Object%20Reference))
  (return 0))

(fn IFGetEquipedWeapon
  (return 0))

(fn IETakeDamage
  (params (BoneName :type Name) (TorsoDamage :type Float%20%28single-precision%29)))

(fn IEDeath)

(fn IFSetSecondaryWeapon
  (params (secondaryWeapon :type A%20Base%20Weapon%20Object%20Reference))
  (return 0))

(fn IFGetSecondaryWeapon
  (return 0))

(fn IETakeDroppedItem
  (params (Item :type Actor%20Object%20Reference)))

(fn IEDropWeapon
  (params (Weapon%20type :type Integer)))