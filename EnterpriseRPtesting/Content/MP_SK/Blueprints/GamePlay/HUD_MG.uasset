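; Multiplayer HUD Blueprint that creates, shows and hides widgets for team and Last Man Standing (battle royale) modes.
; Events drive the health/ammo HUD, observer views, scoreboards, winner and barrier messages, alive count, and a timed kill log.
; Scoreboards are refilled from GameState's PlayerArray, read through interface calls and ordered by repeatedly extracting the maximum score or kills.
; The winner message disables player input, and hiding it retries until the character is valid to re-enable it.
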(event Custom|E_ShowScoreboard
  ;[0.2123 1 0] ScoreBoard Events
  (if (> (Utilities|Time|GetGameTimeinSeconds) 2.0)
    (bind (_redpssorted _bluepssorted) (ScoreBoard|FSortPlayersbyScore))
    (bind _scoreboardwb (ScoreBoard|FCreateScoreBoard _redpssorted _bluepssorted))
    (UserInterface|Viewport|AddtoViewport _scoreboardwb 0)))

(event Custom|E_ShowFinalScoreboard
  ;[0.9663 0 1] Final ScoreBoard. Shows when match is finished
  (Utilities|FlowControl|Delay 0.2)
  (Viewport|RemoveAllWidgets)
  (bind (_redpssorted _bluepssorted) (ScoreBoard|FSortPlayersbyScore))
  (bind _finalscoreboardwb1 (FinalScoreboard|FCreateFinalScoreBoard _redpssorted _bluepssorted))
  (UserInterface|Viewport|AddtoViewport _finalscoreboardwb1 0))

(event Custom|CL_ShowHUD
  (bind _observerhud (Variables|Default|GetObserverHUD))
  ;[0.981 1 0] Main HUD with player health and ammo
  (Utilities|IsValid _observerhud
    (:Is%20Valid
      (Widget|RemovefromParent _observerhud))
    (:Is%20Not%20Valid
      _))
  (Utilities|IsValid (Variables|Default|GetHUD)
    (:Is%20Valid
      (UserInterface|Viewport|AddtoViewport (Variables|Default|GetHUD) 0))
    (:Is%20Not%20Valid
      (bind _returnvalue (UserInterface|CreateWidget "/Game/MP_SK/UI/InGameHUD/HUD.HUD_C" (Game|GetPlayerController 0)))
      (bind _output_get (Variables|Default|SetHUD _returnvalue))
      (UserInterface|Viewport|AddtoViewport _output_get 0))))

(event Custom|E_ShowLMSObserver
  (params (KillerId :type Integer))
  (bind _hud (Variables|Default|GetHUD))
  ;[1 0 0.2934] Hud eventd for battle Royale mode
  ;;[1 1 1] LMS. Show observer hud
  (Utilities|IsValid _hud
    (:Is%20Valid
      (Widget|RemovefromParent _hud))
    (:Is%20Not%20Valid
      _))
  (bind _returnvalue (UserInterface|CreateWidget "/Game/MP_SK/UI/InGameHUD/LMS/LMS_Observer.LMS_Observer_C" (Game|GetPlayerController 0) KillerId))
  (bind _output_get (Variables|LMS|SetLMSObserver _returnvalue))
  (UserInterface|Viewport|AddtoViewport _output_get 0))

(event Custom|E_ShowKillsLog
  ;[1 0 0.0172] Kills Log
  (bind _returnvalue (UserInterface|CreateWidget "/Game/MP_SK/UI/InGameHUD/KillsLog.KillsLog_C" (Game|GetPlayerController 0)))
  (bind _output_get (Variables|Default|SetKillsLog _returnvalue))
  (UserInterface|Viewport|AddtoViewport _output_get 1))

(event Custom|E_ShowWinnerMessage
  (params (LastWinnerTeamId :type Integer))
  ;[1 1 1] Show winner team message
  (Utilities|FlowControl|Sequence
    (:then_0
      (Utilities|FlowControl|Delay 0.2)
      (Viewport|RemoveAllWidgets))
    (:then_1
      (Utilities|FlowControl|Delay 0.3)
      (bind _returnvalue (UserInterface|CreateWidget "/Game/MP_SK/UI/InGameHUD/Classic_Mode/WinnerMessage.WinnerMessage_C" (Game|GetPlayerController 0) LastWinnerTeamId))
      (bind _output_get (Variables|ClassicMode|SetWinnerMessage _returnvalue))
      (UserInterface|Viewport|AddtoViewport _output_get 0)
      (Input|DisableInput (Game|GetPlayerCharacter 0) (Game|GetPlayerController 0)))))

(event Custom|E_HideScoreboard
  (bind _scoreboard (Variables|Default|GetScoreBoard))
  ;[0.2123 1 0] ScoreBoard Events
  (Utilities|IsValid _scoreboard
    (:Is%20Valid
      (Widget|RemovefromParent _scoreboard))))

(event Custom|E_ShowBarrierMessage
  ;[1 0 0.2934] Hud eventd for battle Royale mode
  ;;[1 1 1] LMS. Barrier status
  (bind _returnvalue (UserInterface|CreateWidget "/Game/MP_SK/UI/InGameHUD/LMS/BarrierMessage.BarrierMessage_C" (Game|GetPlayerController 0)))
  (bind _output_get (Variables|LMS|SetBarrierMessage _returnvalue))
  (UserInterface|Viewport|AddtoViewport _output_get 0))

(event Custom|E_ShowLMSScoreBoard
  (params (ShowWinner :type Boolean))
  ;[1 0 0.2934] Hud eventd for battle Royale mode
  ;;[1 1 1] LMS ScoreBoard
  (if (> (Utilities|Time|GetGameTimeinSeconds) 2.0)
    (bind _players_ps_sorted (LMS|FSortPlayersbyKillsLMS))
    (LMS|FCreateScoreBoardLMS _players_ps_sorted ShowWinner)
    (UserInterface|Viewport|AddtoViewport (Variables|LMS|GetLMS_Scoreboard) 0)))

(event Custom|E_Show_PlayersAliveWB
  ;[1 0 0.2934] Hud eventd for battle Royale mode
  ;;[1 1 1] Alive players count widget
  (bind _returnvalue (UserInterface|CreateWidget "/Game/MP_SK/UI/InGameHUD/LMS/PlayersAlive.PlayersAlive_C" (Game|GetPlayerController 0)))
  (UserInterface|Viewport|AddtoViewport _returnvalue 2))

(event Custom|E_ShowObserverHUD
  (params (KillerId :type Integer))
  (bind _hud (Variables|Default|GetHUD))
  ;[0 0.6226 1] Observer HUD
  (Utilities|IsValid _hud
    (:Is%20Valid
      (Widget|RemovefromParent _hud))
    (:Is%20Not%20Valid
      _))
  (bind _returnvalue (UserInterface|CreateWidget "/Game/MP_SK/UI/InGameHUD/ObserverHUD.ObserverHUD_C" (Game|GetPlayerController 0) KillerId))
  (bind _output_get (Variables|Default|SetObserverHUD _returnvalue))
  (UserInterface|Viewport|AddtoViewport _output_get 0))

(event Custom|CL_HideWinnerMessage
  (bind _returnvalue (Game|GetPlayerCharacter 0))
  (bind _winnermessage (Variables|ClassicMode|GetWinnerMessage))
  ;[1 1 1] Hide winner team message
  (Utilities|IsValid _winnermessage
    (:Is%20Valid
      (Widget|RemovefromParent _winnermessage)
      (Utilities|IsValid _returnvalue :!label _label
        (:Is%20Valid
          (Input|EnableInput _returnvalue (Game|GetPlayerController 0)))
        (:Is%20Not%20Valid
          (Utilities|FlowControl|Delay 0.2)
          (goto _label))))))

(event Custom|E_HideObserverHUD
  (bind _observerhud (Variables|Default|GetObserverHUD))
  ;[0 0.6226 1] Observer HUD
  (Utilities|IsValid _observerhud
    (:Is%20Valid
      (Widget|RemovefromParent _observerhud))))

(event Custom|E_HideLMSScoreBoard
  (bind _lms_scoreboard (Variables|LMS|GetLMS_Scoreboard))
  ;[1 0 0.2934] Hud eventd for battle Royale mode
  ;;[1 1 1] LMS ScoreBoard
  (Utilities|IsValid _lms_scoreboard
    (:Is%20Valid
      (Widget|RemovefromParent _lms_scoreboard))))

(event Custom|E_AddKillsLogMessage
  (params (KIllerId :type Integer) (VictimId :type Integer) (HeadShot :type Boolean) (KillerWeapon :type Slate%20Brush%20Structure))
  (bind _killslog (Variables|Default|GetKillsLog))
  (bind _killslogscrollbox (Variables|/Game/MP_SK/UI/InGameHUD/KillsLog.KillsLog_C|GetKillsLogScrollBox _killslog))
  ;[1 0 0.0172] Kills Log
  (bind _returnvalue (UserInterface|CreateWidget "/Game/MP_SK/UI/InGameHUD/KillsLog_Message.KillsLog_Message_C" (Game|GetPlayerController 0) KIllerId VictimId HeadShot KillerWeapon))
  (Utilities|IsValid _killslog
    (:Is%20Valid
      (Widget|Panel|AddChild _killslogscrollbox _returnvalue)
      (Class|ScrollBox|ScrolltoEnd _killslogscrollbox)
      (if (> (Class|PanelWidget|GetChildrenCount _killslogscrollbox) 0) :!label _label
        (Utilities|FlowControl|Delay 4.0)
        (Class|PanelWidget|RemoveChildat _killslogscrollbox)
        (goto _label)))))

(fn FSortPlayersbyScore
  (bind _redteamps (LocalVariables|GetRedTeamPS))
  (bind _redteamscore (LocalVariables|GetRedTeamScore))
  (bind _blueteamscore (LocalVariables|GetBlueTeamScore))
  (bind _blueteamps (LocalVariables|GetBlueTeamPS))
  (bind _indexofmaxvalue (Math|Integer|MaxOfIntArray _blueteamscore))
  (bind _indexofmaxvalue_2 (Math|Integer|MaxOfIntArray _redteamscore))
  (for _array_element (Variables|/Script/Engine.GameStateBase|GetPlayerArray (Game|GetGameState))
    (bind _team (Class|BasePS|IFGetTeam(Message) _array_element))
    (bind _player_score (Class|BasePS|IFGetScore(Message) _array_element))
    (if (== _team 0)
      (Utilities|Array|Add (LocalVariables|GetRedTeamPS) _array_element)
      (Utilities|Array|Add (LocalVariables|GetRedTeamScore) _player_score)
      (else
        (Utilities|Array|Add (LocalVariables|GetBlueTeamPS) _array_element)
        (Utilities|Array|Add (LocalVariables|GetBlueTeamScore) _player_score))))
  (while (> (Utilities|Array|Length (LocalVariables|GetRedTeamPS)) 0)
    (Utilities|Array|Add (LocalVariables|GetRedTeamSorted) (Utilities|Array|Get(acopy) _redteamps _indexofmaxvalue_2))
    (Utilities|Array|RemoveIndex _redteamps _indexofmaxvalue_2)
    (Utilities|Array|RemoveIndex _redteamscore _indexofmaxvalue_2))
  (while (> (Utilities|Array|Length (LocalVariables|GetBlueTeamPS)) 0)
    (Utilities|Array|Add (LocalVariables|GetBlueTeamSorted) (Utilities|Array|Get(acopy) _blueteamps _indexofmaxvalue))
    (Utilities|Array|RemoveIndex _blueteamps _indexofmaxvalue)
    (Utilities|Array|RemoveIndex _blueteamscore _indexofmaxvalue))
  (return (LocalVariables|GetRedTeamSorted) (LocalVariables|GetBlueTeamSorted)))

(fn FCreateScoreBoard
  (params (RedPSSorted :type Array%20of%20Player%20State%20Object%20References) (BluePSSorted :type Array%20of%20Player%20State%20Object%20References))
  (bind _returnvalue (Game|GetPlayerController 0))
  (Utilities|IsValid (Variables|Default|GetScoreboard)
    (:Is%20Valid
      _)
    (:Is%20Not%20Valid
      ;[1 1 1] Create Scoreboard if not exist
      (bind _returnvalue_2 (UserInterface|CreateWidget "/Game/MP_SK/UI/InGameHUD/ScoreBoard.ScoreBoard_C" (Game|GetPlayerController 0)))
      (Variables|Default|SetScoreBoard _returnvalue_2)))
  (Utilities|FlowControl|Sequence
    (:then_0
      (Widget|Panel|ClearChildren (Variables|/Game/MP_SK/UI/InGameHUD/ScoreBoard.ScoreBoard_C|GetBlueTeamPlayersList (Variables|Default|GetScoreBoard))))
    (:then_1
      ;[1 1 1] Add player line widget in Red or blue ScrollBox in Scoreboard
      (for _array_element RedPSSorted
        (bind _returnvalue_3 (UserInterface|CreateWidget "/Game/MP_SK/UI/InGameHUD/ScoreBoard_PlayerLine.ScoreBoard_PlayerLine_C" _returnvalue (Variables|/Script/Engine.PlayerState|GetPlayerId _array_element)))
        (Widget|Panel|AddChild (Variables|/Game/MP_SK/UI/InGameHUD/ScoreBoard.ScoreBoard_C|GetRedTeamPlayersList (Variables|Default|GetScoreBoard)) _returnvalue_3))
      (for _array_element_2 BluePSSorted
        (bind _returnvalue_4 (UserInterface|CreateWidget "/Game/MP_SK/UI/InGameHUD/ScoreBoard_PlayerLine.ScoreBoard_PlayerLine_C" _returnvalue (Variables|/Script/Engine.PlayerState|GetPlayerId _array_element_2)))
        (Widget|Panel|AddChild (Variables|/Game/MP_SK/UI/InGameHUD/ScoreBoard.ScoreBoard_C|GetBlueTeamPlayersList (Variables|Default|GetScoreBoard)) _returnvalue_4))
      (return (Variables|Default|GetScoreboard)))))

(fn FCreateFinalScoreBoard
  (params (RedTEamPS :type Array%20of%20Player%20State%20Object%20References) (BlueTeamPS :type Array%20of%20Player%20State%20Object%20References))
  (bind _returnvalue (Game|GetPlayerController 0))
  (Utilities|FlowControl|Sequence
    (:then_0
      (bind _returnvalue_2 (UserInterface|CreateWidget "/Game/MP_SK/UI/InGameHUD/FinalScoreboard.FinalScoreboard_C" (Game|GetPlayerController 0)))
      (Variables|Default|SetFinalScoreboard _returnvalue_2))
    (:then_1
      (Widget|Panel|ClearChildren (Variables|/Game/MP_SK/UI/InGameHUD/FinalScoreboard.FinalScoreboard_C|GetRedTeamPlayersList (Variables|Default|GetFinalScoreboard))))
    (:then_2
      (for _array_element RedTEamPS
        (bind _returnvalue_3 (UserInterface|CreateWidget "/Game/MP_SK/UI/InGameHUD/ScoreBoard_PlayerLine.ScoreBoard_PlayerLine_C" _returnvalue (Variables|/Script/Engine.PlayerState|GetPlayerId _array_element)))
        (Widget|Panel|AddChild (Variables|/Game/MP_SK/UI/InGameHUD/FinalScoreboard.FinalScoreboard_C|GetRedTeamPlayersList (Variables|Default|GetFinalScoreboard)) _returnvalue_3))
      (for _array_element_2 BlueTeamPS
        (bind _returnvalue_4 (UserInterface|CreateWidget "/Game/MP_SK/UI/InGameHUD/ScoreBoard_PlayerLine.ScoreBoard_PlayerLine_C" _returnvalue (Variables|/Script/Engine.PlayerState|GetPlayerId _array_element_2)))
        (Widget|Panel|AddChild (Variables|/Game/MP_SK/UI/InGameHUD/FinalScoreboard.FinalScoreboard_C|GetBlueTeamPlayersList (Variables|Default|GetFinalScoreboard)) _returnvalue_4))
      (return (Variables|Default|GetFinalScoreboard)))))

(fn FSortPlayersbyKillsLMS
  (bind _playersps (LocalVariables|GetPlayersPS))
  (bind _playerskills (LocalVariables|GetPlayersKills))
  (bind _indexofmaxvalue (Math|Integer|MaxOfIntArray _playerskills))
  (for _array_element (Variables|/Script/Engine.GameStateBase|GetPlayerArray (Game|GetGameState))
    (bind _kills (Class|BasePS|IFGetKills(Message) _array_element))
    (Utilities|Array|Add (LocalVariables|GetPlayersPS) _array_element)
    (Utilities|Array|Add (LocalVariables|GetPlayersKills) _kills))
  (while (> (Utilities|Array|Length (LocalVariables|GetPlayersPS)) 0)
    (Utilities|Array|Add (LocalVariables|GetPlayersPSSorted) (Utilities|Array|Get(acopy) _playersps _indexofmaxvalue))
    (Utilities|Array|RemoveIndex _playersps _indexofmaxvalue)
    (Utilities|Array|RemoveIndex _playerskills _indexofmaxvalue))
  (return (LocalVariables|GetPlayersPSSorted)))

(fn FCreateScoreBoardLMS
  (params (PlayersPSSorted :type Array%20of%20Player%20State%20Object%20References) (ShowWinner :type Boolean))
  (Utilities|IsValid (Variables|LMS|GetLMS_Scoreboard)
    (:Is%20Valid
      _)
    (:Is%20Not%20Valid
      ;[1 1 1] Create Scoreboard if not exist
      (bind _returnvalue (UserInterface|CreateWidget "/Game/MP_SK/UI/InGameHUD/LMS/LMS_ScoreBoard.LMS_ScoreBoard_C" (Game|GetPlayerController 0) ShowWinner))
      (Variables|LMS|SetLMS_Scoreboard _returnvalue)))
  (Utilities|FlowControl|Sequence
    (:then_0
      (Widget|Panel|ClearChildren (Variables|/Game/MP_SK/UI/InGameHUD/LMS/LMS_ScoreBoard.LMS_ScoreBoard_C|GetPlayersScrollBox (Variables|LMS|GetLMS_Scoreboard)))
      (Variables|/Game/MP_SK/UI/InGameHUD/LMS/LMS_ScoreBoard.LMS_ScoreBoard_C|SetShowWinner (Variables|LMS|GetLMS_Scoreboard) ShowWinner))
    (:then_1
      (for _array_element PlayersPSSorted
        (bind _returnvalue_2 (UserInterface|CreateWidget "/Game/MP_SK/UI/InGameHUD/LMS/LMS_ScoreBoard_PlayerLine.LMS_ScoreBoard_PlayerLine_C" (Game|GetPlayerController 0) (Variables|/Script/Engine.PlayerState|GetPlayerId _array_element)))
        (Widget|Panel|AddChild (Variables|/Game/MP_SK/UI/InGameHUD/LMS/LMS_ScoreBoard.LMS_ScoreBoard_C|GetPlayersScrollBox (Variables|LMS|GetLMS_Scoreboard)) _returnvalue_2)))))