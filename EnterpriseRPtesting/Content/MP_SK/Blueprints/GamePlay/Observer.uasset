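; Observer actor for spectating, letting the player cycle the view between pawns with the mouse.
; It enables its own input on begin play, then left and right clicks send interface messages to the player controller to attach it to the next or previous pawn.
; Each tick it copies the player character's control pitch and yaw to its own rotation, since input on the dead pawn is disabled.
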(event EventTick
  (params (DeltaSeconds :type Float%20%28single-precision%29))
  (bind _returnvalue (Game|GetPlayerCharacter 0))
  (bind _returnvalue_2 (Pawn|GetControlRotation _returnvalue :!class /Script/Engine.Pawn))
  ;[1 1 1] We disabled input in dead pawn, so here updates camera rotation
  (Utilities|IsValid _returnvalue
    (:Is%20Valid
      (Transformation|SetActorRotation (Math|Rotator|MakeRotator 0.0 (.pitch _returnvalue_2) (.yaw _returnvalue_2))))))

(event EventBeginPlay
  ;[1 1 1] Enable input in observer on begin play
  (Input|EnableInput (Game|GetPlayerController 0)))

(event Input|MouseEvents|LeftMouseButton
  (params (Key :type Key%20Structure :default "AnyKey"))
  ;[1 0.007639 0] LMB - watch next pawn. RMB - watch prev pawn
  (:Pressed
    (Utilities|IsValid self
      (:Is%20Valid
        (Class|BasePC|IEAttachObservertoNextPawn(Message) (Game|GetPlayerController 0))))))

(event Input|MouseEvents|RightMouseButton
  (params (Key :type Key%20Structure :default "AnyKey"))
  ;[1 0.007639 0] LMB - watch next pawn. RMB - watch prev pawn
  (:Pressed
    (Utilities|IsValid self
      (:Is%20Valid
        (Class|BasePC|IEAttachObservertoPrevPawn(Message) (Game|GetPlayerController 0))))))

(fn ConstructionScript)